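; Player controller for a map view that pans the camera pawn by mouse drag and focuses it on selected map actors.
; While PanCamera is held, Tick moves the pawn by the mouse delta, clamped to X/Y limits, unless focusing.
; FocusOnObject uses a timeline to lerp the pawn to an offset, re-pitched view, then shows the building info widget.
; BackToDefaultPosition removes the widget and lerps back to the starting transform, re-enabling panning.
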(event `BackToDefaultPosition`
  ;[1 1 1] Move Camera To Default Position
  (`Widget.RemoveFromParent` (`self.InfoWidget`))
  (`self.SaveCurrentLocationAndRotation`)
  (bind (_direction _animcurve) (`Timeline|BackToDefault` :!via `PlayFromStart`)
    (:`Update`
      (`self.K2_SetActorLocationAndRotation` (`self.K2_GetPawn`) (`KismetMathLibrary.VLerp` (`self.CurrentLocation`) (`self.StartLocation`) _animcurve) (`KismetMathLibrary.RLerp` (`self.CurrentRotation`) (`self.StartRotation`) _animcurve) false false))
    (:`Finished`
      (set `self.IsFocusing` false))))

(event `FocusOnObject`
  (params (FocusActor :type "Actor Object Reference"))
  (bind _infowidget (`self.InfoWidget`))
  ;[1 1 1] Focus Camera On Selected Object. When focused - show widget with Info.
  (`/Engine/EditorBlueprintResources/StandardMacros.IsValid` FocusActor
    (:`Is Valid`
      (if (not (`self.IsFocusing`))
        (set `self.IsFocusing` true)
        (`self.SaveCurrentLocationAndRotation`)
        (`self.CalculateTargetLocationAndRotation` FocusActor)
        (bind (_direction _animcurve) (`Timeline|FocusCamera` :!via `PlayFromStart`)
          (:`Update`
            (`self.K2_SetActorLocationAndRotation` (`self.K2_GetPawn`) (`KismetMathLibrary.VLerp` (`self.CurrentLocation`) (`self.TargetLocation`) _animcurve) (`KismetMathLibrary.RLerp` (`self.CurrentRotation`) (`self.TargetRotation`) _animcurve) false false))
          (:`Finished`
            (`/Game/ImmersionTest/Blueprints/WBP_BuildingInfo.SetAllValues` _infowidget (cast `/Game/ImmersionTest/Blueprints/BP_MapActorBase` FocusActor :!pure true))
            (`UserWidget.AddToViewport` _infowidget 0)))))))

(event `self.ReceiveBeginPlay`
  (bind _returnvalue (`self.K2_GetPawn`))
  (bind _returnvalue_2 (`|CreateWidget` "/Game/ImmersionTest/Blueprints/WBP_BuildingInfo.WBP_BuildingInfo_C" self))
  (set `self.InfoWidget` _returnvalue_2)
  ;[1 1 1] Saving start location and rotation camera values
  (set `self.StartRotation` (`self.K2_GetActorRotation` _returnvalue))
  (set `self.StartLocation` (`self.K2_GetActorLocation` _returnvalue)))

(event `self.ReceiveTick`
  (params (DeltaSeconds :type "Float (single-precision)"))
  ;[1 1 1] Prevent camera movement while focusing
  (if (not (`self.IsFocusing`))
    (`self.UpdateCameraLocation`)))

(event `UpdateCameraLocation`
  (bind (_locationx _locationy) (`self.GetMousePosition`))
  (if (`self.IsSwipingCamera`)
    (`self.K2_SetActorLocation` (`self.K2_GetPawn`) (`self.GetDeltaLocation`) false false)
    (set `self.LastPosX` _locationx)
    (set `self.LastPosY` _locationy)))

(event `InputAction|PanCamera`
  (params (Key :type "Key Structure"))
  (bind (_locationx _locationy) (`self.GetMousePosition`))
  ;[1 1 1] Get mouse input
  (:`Pressed`
    (set `self.IsSwipingCamera` true)
    (set `self.LastPosX` _locationx)
    (set `self.LastPosY` _locationy))
  (:`Released`
    (set `self.IsSwipingCamera` false)))

(fn `CalculateTargetLocationAndRotation`
  (params (self2 :type "Actor Object Reference"))
  (bind (_startrotation_roll _startrotation_pitch _startrotation_yaw) (`KismetMathLibrary.BreakRotator` (`self.StartRotation`)))
  (set `self.TargetLocation` (+ (`self.K2_GetActorLocation` self2) (`self.FocusOffset`)))
  (set `self.TargetRotation` (`KismetMathLibrary.MakeRotator` _startrotation_roll (+ _startrotation_pitch 50.0) _startrotation_yaw)))

(fn `GetDeltaLocation`
  (returns (ReturnValue :type "Vector Structure"))
  (bind (_locationx _locationy) (`self.GetMousePosition`))
  (bind _limitx (`self.LimitX`))
  (bind _limity (`self.LimitY`))
  (bind (_returnvalue_x _returnvalue_y _returnvalue_z) (`KismetMathLibrary.BreakVector` (`self.K2_GetActorLocation` (`self.K2_GetPawn`))))
  ;[1 1 1] Getting mouse position and calculating delta position for camera movement
  (return (`KismetMathLibrary.MakeVector` (`KismetMathLibrary.FClamp` (+ (* (- (`self.LastPosX`) _locationx) 100.0) _returnvalue_x) (* _limitx -1.0) _limitx) (`KismetMathLibrary.FClamp` (+ (* (- (`self.LastPosY`) _locationy) 100.0) _returnvalue_y) (* _limity -1.0) _limity) _returnvalue_z)))

(fn `SaveCurrentLocationAndRotation`
  (set `self.CurrentRotation` (`self.K2_GetActorRotation` (`self.K2_GetPawn`)))
  (set `self.CurrentLocation` (`self.K2_GetActorLocation` (`self.K2_GetPawn`))))

(fn `UserConstructionScript`)